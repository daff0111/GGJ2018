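; Robot character Blueprint that starts its StateMachine and presents the sequence through automatically switching cameras.
; StartStateMachine adds BP_TestUI, disables capsule gravity and collision, then a self-rearming timer blends to random cameras every few seconds.
; Tick watches for state 7 to stop switching and lock the view onto VCam.
; Game over enables physics simulation on the mesh after a delay; Deactivate hides the mesh.
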(event Custom|Deactivate
  (Rendering|SetVisibility (Variables|Character|GetMesh) false false))

(event Custom|StartStateMachine
  (bind _capsulecomponent (Variables|Default|GetCapsuleComponent))
  (bind _camera (Variables|Default|GetCamera))
  (bind _returnvalue (UserInterface|CreateWidget "/Game/Gameplay/UI/BP_TestUI.BP_TestUI_C"))
  (UserInterface|Viewport|AddtoViewport _returnvalue 0)
  (Class|StateMachine|Start (Variables|Default|GetStateMachine))
  (Physics|SetEnableGravity _capsulecomponent false)
  (EventDispatchers|BindEventtoGameOverDelegate (Variables|Default|GetStateMachine) (delegate Custom|OnGameOver))
  (Collision|SetCollisionEnabled _capsulecomponent "NoCollision")
  ;[1 1 1] Camera Switch
  (Game|Player|SetViewTargetwithBlend (Game|GetPlayerController 0) (Utilities|Array|Get(acopy) _camera (Math|Random|RandomIntegerinRange 0 (- (Utilities|Array|Length _camera) 1))) 2.0 "VTBlend_Cubic" 0.0 true)
  (bind _returnvalue_2 (Utilities|Time|SetTimerbyEvent (delegate Custom|CameraSwitch) (Math|Random|RandomFloatinRange 2.0 4.0)))
  (Variables|Default|SetCameraTimer _returnvalue_2))

(event Custom|OnGameOver
  (params (Victory :type Boolean))
  ;[1 1 1] On Game End
  (bind _returnvalue (Utilities|Time|SetTimerbyEvent (delegate Custom|GameOverEventTimer) 5.0))
  (Variables|Default|SetGameOverTimer _returnvalue))

(event Custom|GameOverEventTimer
  ;[1 1 1] On Game End
  (Physics|SetSimulatePhysics (Variables|Character|GetMesh) true))

(event Custom|CameraSwitch
  (bind _camera (Variables|Default|GetCamera))
  ;[1 1 1] Camera Switch
  (if (not (Variables|Default|GetFinalCameraLock))
    (Game|Player|SetViewTargetwithBlend (Game|GetPlayerController 0) (Utilities|Array|Get(acopy) _camera (Math|Random|RandomIntegerinRange 0 (- (Utilities|Array|Length _camera) 1))) 2.0 "VTBlend_Cubic" 0.0 true)
    (bind _returnvalue (Utilities|Time|SetTimerbyEvent (delegate Custom|CameraSwitch) (Math|Random|RandomFloatinRange 2.0 4.0)))
    (Variables|Default|SetCameraTimer _returnvalue)
    (else
      (Utilities|Time|ClearandInvalidateTimerbyHandle (Variables|Default|GetCameraTimer)))))

(event EventTick
  (params (DeltaSeconds :type Float%20%28single-precision%29))
  (if (and (== (Variables|/Script/TRANSmission.StateMachine|GetCurrentState (Variables|Default|GetStateMachine)) 7) (not (Variables|Default|GetFinalCameraLock)))
    (Utilities|Time|ClearandInvalidateTimerbyHandle (Variables|Default|GetCameraTimer))
    (Game|Player|SetViewTargetwithBlend (Game|GetPlayerController 0) (Variables|Default|GetVCam) 2.0 "VTBlend_Cubic" 1.0 true)
    (Variables|Default|SetFinalCameraLock true)))

(event Collision|EventActorBeginOverlap
  (params (OtherActor :type Actor%20Object%20Reference)))

(fn ConstructionScript)